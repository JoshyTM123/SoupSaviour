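; BP_FallingIcicle is a hazard actor that drops an icicle cone after the player character enters its trigger box.
; BeginPlay caches the cone's world transform.
; An overlap by BP_ThirdPersonCharacter waits briefly, enables physics simulation so the cone falls, then after a further delay disables physics and snaps the cone back to its start, ready to fall again.
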(event OnComponentBeginOverlap(Box)
  (params (OverlappedComponent :type Primitive%20Component%20Object%20Reference) (OtherActor :type Actor%20Object%20Reference) (OtherComp :type Primitive%20Component%20Object%20Reference) (OtherBodyIndex :type Integer) (bFromSweep :type Boolean) (SweepResult :type Hit%20Result%20Structure%20%28by%20ref%29))
  (Utilities|Casting|CastToBP_ThirdPersonCharacter OtherActor)
  (Utilities|FlowControl|Delay 0.7)
  (Physics|SetSimulatePhysics (Variables|Default|GetCone) true)
  (Utilities|FlowControl|Delay 1.0)
  (Physics|SetSimulatePhysics (Variables|Default|GetCone) false)
  (Transformation|SetWorldLocationAndRotation (Variables|Default|GetCone) (Variables|Default|GetStartingPos) (Variables|Default|GetStartingRot) false false))

(event EventBeginPlay
  (bind _cone (Variables|Default|GetCone))
  (Variables|Default|SetStartingPos (Transformation|GetWorldLocation _cone))
  (Variables|Default|SetStartingRot (Transformation|GetWorldRotation _cone)))

(fn ConstructionScript)