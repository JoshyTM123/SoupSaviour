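; BP_ChangingPlant is a plant made of a stem and two leaves, meant to stay hidden until a sprinkler activates it.
; BeginPlay and Activate both toggle part visibility through an IsVisibile flag, then set collision from that flag.
; HasActivated limits Activate to a single toggle.
; Showing the plant re-enables collision only on the leaves, while hiding it disables collision on all three parts.
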(event Custom|Activate
  ;[0.15 0.15 0.15 0.5] Not visible until sprinkler has been activated
  (if (not (Variables|Default|GethasActivated))
    (CallFunction|ChangeVisibility)
    (CallFunction|ChangeCollision)
    (Variables|Default|SethasActivated true)))

(event EventBeginPlay
  ;[0.15 0.15 0.15 0.5] Not visible until sprinkler has been activated
  (CallFunction|ChangeVisibility)
  (CallFunction|ChangeCollision))

(fn ConstructionScript)

(fn ChangeVisibility
  (if (Variables|Default|GetisVisibile)
    (Rendering|SetVisibility (Variables|Default|GetLeaf) false false)
    (Rendering|SetVisibility (Variables|Default|GetLeaf2) false false)
    (Rendering|SetVisibility (Variables|Default|GetStem) false false)
    (Variables|Default|SetisVisibile false)
    (else
      (Rendering|SetVisibility (Variables|Default|GetLeaf) true false)
      (Rendering|SetVisibility (Variables|Default|GetLeaf2) true false)
      (Rendering|SetVisibility (Variables|Default|GetStem) true false)
      (Variables|Default|SetisVisibile true))))

(fn ChangeCollision
  (if (Variables|Default|GetisVisibile)
    (Collision|SetCollisionEnabled (Variables|Default|GetLeaf) "QueryAndPhysics")
    (Collision|SetCollisionEnabled (Variables|Default|GetLeaf2) "QueryAndPhysics")
    (else
      (Collision|SetCollisionEnabled (Variables|Default|GetStem) "NoCollision")
      (Collision|SetCollisionEnabled (Variables|Default|GetLeaf) "NoCollision")
      (Collision|SetCollisionEnabled (Variables|Default|GetLeaf2) "NoCollision"))))