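; Poster is an interactable Blueprint that shows a full-screen poster or letter widget when the player interacts with it.
; On BeginPlay it creates the poster widget and an "open letter" prompt widget, which appears while the third-person character overlaps its Box.
; Interact toggles the poster through a FlipFlop, and leaving the Box removes both widgets without resetting the toggle state.
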(event OnComponentEndOverlap(Box)
  (params (OverlappedComponent :type Primitive%20Component%20Object%20Reference) (OtherActor :type Actor%20Object%20Reference) (OtherComp :type Primitive%20Component%20Object%20Reference) (OtherBodyIndex :type Integer))
  (Utilities|Casting|CastToBP_ThirdPersonCharacter OtherActor)
  (CallFunction|PosterOff)
  (Widget|RemovefromParent (Variables|Default|GetInteractWidget)))

(event OnComponentBeginOverlap(Box)
  (params (OverlappedComponent :type Primitive%20Component%20Object%20Reference) (OtherActor :type Actor%20Object%20Reference) (OtherComp :type Primitive%20Component%20Object%20Reference) (OtherBodyIndex :type Integer) (bFromSweep :type Boolean) (SweepResult :type Hit%20Result%20Structure%20%28by%20ref%29))
  (Utilities|Casting|CastToBP_ThirdPersonCharacter OtherActor)
  (UserInterface|Viewport|AddtoViewport (Variables|Default|GetInteractWidget) 0))

(event Custom|PosterOff
  ;[0.15 0.15 0.15 0.5] Displays or remove poster image from screen
  (if (UserInterface|Viewport|IsinViewport (Variables|Default|GetPosterWidget))
    (Widget|RemovefromParent (Variables|Default|GetPosterWidget))))

(event Custom|PosterOn
  ;[0.15 0.15 0.15 0.5] Displays or remove poster image from screen
  (if (not (UserInterface|Viewport|IsinViewport (Variables|Default|GetPosterWidget)))
    (UserInterface|Viewport|AddtoViewport (Variables|Default|GetPosterWidget) 0)))

(event EventBeginPlay
  (bind _returnvalue (UserInterface|CreateWidget "/Game/Widgets/W_Poster.W_Poster_C"))
  (Variables|Default|SetPosterWidget _returnvalue)
  (bind _returnvalue_2 (UserInterface|CreateWidget "/Game/Widgets/W_Interact.W_Interact_C"))
  (bind _output_get (Variables|Default|SetInteractWidget _returnvalue_2))
  (Variables|/Game/Widgets/W_Interact.W_Interact_C|SetPromptText _output_get "Press E to Open Letter"))

(event EventInteract
  (Utilities|FlowControl|FlipFlop
    (:A
      (CallFunction|Posteron))
    (:B
      (CallFunction|PosterOff))))

(fn ConstructionScript)

(fn ReturnText
  (return ""))