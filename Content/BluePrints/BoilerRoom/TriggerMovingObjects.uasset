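; A one-shot trigger volume in the BoilerRoom folder that sets level objects moving when the player character walks into it.
; Box overlap casts to BP_ThirdPersonCharacter and passes through a DoOnce, so only the first valid overlap fires.
; The ForVent and ForSpikes flags choose whether MoveObject is called on the vent reference, every spike in an array, or a single object reference, with vent taking priority.
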(event OnComponentBeginOverlap(Box)
  (params (OverlappedComponent :type Primitive%20Component%20Object%20Reference) (OtherActor :type Actor%20Object%20Reference) (OtherComp :type Primitive%20Component%20Object%20Reference) (OtherBodyIndex :type Integer) (bFromSweep :type Boolean) (SweepResult :type Hit%20Result%20Structure%20%28by%20ref%29))
  (Utilities|Casting|CastToBP_ThirdPersonCharacter OtherActor)
  (Utilities|FlowControl|DoOnce false
    (:Completed
      (if (Variables|Default|GetforVent)
        (Default|MoveObject (Variables|Default|GetventRef))
        (elif (Variables|Default|GetForSpikes)
          (for _array_element (Variables|Default|GetArrayOfSpikes)
            (Default|MoveObject _array_element))
          (else
            (Default|MoveObject (Variables|Default|GetobjectRef))))))))

(fn ConstructionScript)