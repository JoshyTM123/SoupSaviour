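; BP_MovingNail is a moving hazard that shuttles along a referenced spline and respawns the player at a checkpoint on touch.
; MoveObject makes its three meshes glow purple, waits, then plays a timeline scaled to the set travel time.
; The timeline moves the actor by spline distance, pausing at each end before reversing direction.
; Overlapping the death box triggers RespawnAtCheckpoint on the third-person character.
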(event OnComponentBeginOverlap(DeaathBox)
  (params (OverlappedComponent :type Primitive%20Component%20Object%20Reference) (OtherActor :type Actor%20Object%20Reference) (OtherComp :type Primitive%20Component%20Object%20Reference) (OtherBodyIndex :type Integer) (bFromSweep :type Boolean) (SweepResult :type Hit%20Result%20Structure%20%28by%20ref%29))
  (bind _asbp_third_person_character (Utilities|Casting|CastToBP_ThirdPersonCharacter OtherActor))
  (Default|RespawnatCheckpoint _asbp_third_person_character))

(event Custom|Move%20Object
  (bind _spline_ref (Variables|Default|GetSpline%20Ref))
  (bind _timedelay (Variables|Default|GettimeDelay))
  (bind _spline (Variables|/Game/BluePrints/BoilerRoom/BP_SplinePath.BP_SplinePath_C|GetSpline _spline_ref))
  (Rendering|Material|SetMaterial (Variables|Default|GetSphere) 0 "/Game/CustomMaterials/PurpleGlow.PurpleGlow")
  (Utilities|FlowControl|Delay (Variables|Default|GettimeDelay))
  (Components|Timeline|SetPlayRate (Variables|Default|GetT_Move) (/ 1.0 (Variables|Default|GettimeToComplete)))
  (bind _move_track (Timeline|T_Move Play)
    (:Update
      (Transformation|SetActorLocation (Spline|GetLocationatDistanceAlongSpline _spline (Math|Float|Lerp 0.0 (Spline|GetSplineLength _spline) _move_track) "World") false false))
    (:Finished
      (if (Variables|Default|GetisMovingForward)
        (Utilities|FlowControl|Delay _timedelay)
        (Utilities|String|Reverse (Variables|Default|GetT_Move))
        (Variables|Default|SetisMovingForward false)
        (else
          (Utilities|FlowControl|Delay _timedelay)
          (Audio|Components|Audio|Play (Variables|Default|GetT_Move))
          (Variables|Default|SetisMovingForward true))))))

(fn ConstructionScript)