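; BP_Cauldron is the boiler room cauldron the player uses to finish the soup, triggering an end cutscene.
; While IsSnapped is set, a box overlap shows or hides a "Finish the Soup" prompt widget for the player.
; Interacting when snapped hides the player and plays a referenced level sequence, then adds the end-cutscene widget after the sequence's duration elapses.
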(event OnComponentBeginOverlap(Box)
  (params (OverlappedComponent :type Primitive%20Component%20Object%20Reference) (OtherActor :type Actor%20Object%20Reference) (OtherComp :type Primitive%20Component%20Object%20Reference) (OtherBodyIndex :type Integer) (bFromSweep :type Boolean) (SweepResult :type Hit%20Result%20Structure%20%28by%20ref%29))
  ;[0.15 0.15 0.15 0.5] Display Widget
  (if (and (== OtherActor (Game|GetPlayerCharacter 0)) (Variables|Default|GetisSnapped))
    (UserInterface|Viewport|AddtoViewport (Variables|Default|GetInteractWidget) 0)))

(event OnComponentEndOverlap(Box)
  (params (OverlappedComponent :type Primitive%20Component%20Object%20Reference) (OtherActor :type Actor%20Object%20Reference) (OtherComp :type Primitive%20Component%20Object%20Reference) (OtherBodyIndex :type Integer))
  ;[0.15 0.15 0.15 0.5] Display Widget
  (if (and (== (Game|GetPlayerCharacter 0) OtherActor) (Variables|Default|GetisSnapped))
    (Widget|RemovefromParent (Variables|Default|GetInteractWidget))))

(event EventBeginPlay
  ;[0.15 0.15 0.15 0.5] Display Widget
  (bind _returnvalue (UserInterface|CreateWidget "/Game/Widgets/W_Interact.W_Interact_C"))
  (bind _output_get (Variables|Default|SetInteractWidget _returnvalue))
  (Variables|/Game/Widgets/W_Interact.W_Interact_C|SetPromptText _output_get "Finish the Soup"))

(event EventInteract
  (bind _levsequenceref (Variables|Default|GetlevSequenceRef))
  (bind _sequenceplayer (Variables|/Script/LevelSequence.LevelSequenceActor|GetSequencePlayer _levsequenceref))
  (if (Variables|Default|GetisSnapped)
    (Rendering|SetActorHiddenInGame (Game|GetPlayerCharacter 0) true)
    (Sequencer|Player|Play _sequenceplayer :!class /Script/MovieScene.MovieSceneSequencePlayer)
    (Utilities|FlowControl|Delay (Class|TimeManagementBlueprintLibrary|ToSeconds(QualifiedFrameTime) (Media|MediaPlayer|GetDuration _sequenceplayer)))
    (bind _returnvalue (UserInterface|CreateWidget "/Game/Widgets/W_EndCutscene.W_EndCutscene_C"))
    (UserInterface|Viewport|AddtoViewport _returnvalue 0)))

(fn ConstructionScript)

(fn ReturnText
  (return ""))