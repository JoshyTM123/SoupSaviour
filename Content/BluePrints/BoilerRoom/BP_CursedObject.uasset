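; BP_CursedObject is an actor whose mesh glows purple and shuttles back and forth along a referenced spline in the Boiler Room.
; MoveObject, optionally called at BeginPlay, applies the glow material, waits, then starts a timeline scaled to a set travel time.
; The timeline lerps distance along the spline to set location, alternately reversing and replaying after a delay at each end.
; The construction script sets the cube's mesh from a variable.
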(event Custom|Move%20Object
  (bind _splineref (Variables|Default|GetsplineRef))
  (bind _timedelay (Variables|Default|GettimeDelay))
  (bind _spline (Variables|/Game/BluePrints/BoilerRoom/BP_SplinePath.BP_SplinePath_C|GetSpline _splineref))
  (Rendering|Material|SetMaterial (Variables|Default|GetCube) 0 "/Game/CustomMaterials/PurpleGlow.PurpleGlow")
  (Utilities|FlowControl|Delay (Variables|Default|GettimeDelay))
  (Components|Timeline|SetPlayRate (Variables|Default|GetT_Move) (/ 1.0 (Variables|Default|GettimeToComplete)))
  (bind _move_track (Timeline|T_Move Play)
    (:Update
      (Transformation|SetActorLocation (Spline|GetLocationatDistanceAlongSpline _spline (Math|Float|Lerp 0.0 (Spline|GetSplineLength _spline) _move_track) "World") false false))
    (:Finished
      (if (Variables|Default|GetisMovingForward)
        (Utilities|FlowControl|Delay _timedelay)
        (Utilities|String|Reverse (Variables|Default|GetT_Move))
        (Variables|Default|SetisMovingForward false)
        (else
          (Utilities|FlowControl|Delay _timedelay)
          (Audio|Components|Audio|Play (Variables|Default|GetT_Move))
          (Variables|Default|SetisMovingForward true))))))

(event EventBeginPlay
  (if (Variables|Default|GetbeginAtStart)
    (CallFunction|MoveObject)))

(fn ConstructionScript
  (Components|StaticMesh|SetStaticMesh (Variables|Default|GetCube) (Variables|Default|GetNew%20Mesh)))