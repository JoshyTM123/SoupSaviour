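; BP_PlateMovement is a Boiler Room moving platform that slides along its relative Y axis when told to go forwards or backwards.
; GoForwards and GoBackwards switch the Platform to a purple glow material, wait for DelayTime, then play or reverse the T_Movement timeline.
; The timeline's Position track sets the Platform's relative location, and its Finished output restores the silver material.
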(event Custom|GoBackwards
  (Rendering|Material|SetMaterial (Variables|Default|GetPlatform) 0 "/Game/CustomMaterials/PurpleGlow.PurpleGlow")
  (Utilities|FlowControl|Delay (Variables|Default|GetDelayTime))
  (bind _position (Timeline|T_Movement Reverse)
    (:Update
      (Transformation|SetRelativeLocation (Variables|Default|GetPlatform) (Math|Vector|MakeVector 0.0 _position 0.0) false false))
    (:Finished
      (Rendering|Material|SetMaterial (Variables|Default|GetPlatform) 0 "/Game/CustomMaterials/Silver.Silver"))))

(event Custom|GoForwards
  (Rendering|Material|SetMaterial (Variables|Default|GetPlatform) 0 "/Game/CustomMaterials/PurpleGlow.PurpleGlow")
  (Utilities|FlowControl|Delay (Variables|Default|GetDelayTime))
  (bind _position (Timeline|T_Movement Play)
    (:Update
      (Transformation|SetRelativeLocation (Variables|Default|GetPlatform) (Math|Vector|MakeVector 0.0 _position 0.0) false false))
    (:Finished
      (Rendering|Material|SetMaterial (Variables|Default|GetPlatform) 0 "/Game/CustomMaterials/Silver.Silver"))))

(fn ConstructionScript)