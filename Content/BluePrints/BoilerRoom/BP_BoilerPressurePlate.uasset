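; BP_BoilerPressurePlate is a boiler room pressure plate that activates when something overlaps its detection component.
; On first overlap it sets IsActive, plays an electric zap, sets IsFilling on the referenced cable and plays a timeline moving the switch along local Z.
; When no overlapping actors remain it clears IsActive and reverses the timeline, but again sets the cable's IsFilling to true.
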(event OnComponentBeginOverlap(OverlaptDetection)
  (params (OverlappedComponent :type Primitive%20Component%20Object%20Reference) (OtherActor :type Actor%20Object%20Reference) (OtherComp :type Primitive%20Component%20Object%20Reference) (OtherBodyIndex :type Integer) (bFromSweep :type Boolean) (SweepResult :type Hit%20Result%20Structure%20%28by%20ref%29))
  (if (not (Variables|Default|GetisActive))
    (Variables|Default|SetisActive true)
    (Audio|PlaySoundatLocation "/Game/Audio/Electric_Zap.Electric_Zap" (Transformation|GetActorLocation) "0, 0, 0" 1.0 1.0 0.0 "/Game/NewSoundAttenuation.NewSoundAttenuation" 0 0 0)
    (Variables|/Game/BluePrints/BoilerRoom/BP_FurnaceCable.BP_FurnaceCable_C|SetisFilling (Variables|Default|GetCableRef) true)
    (bind _newtrack_0 (Timeline|PressureMove Play)
      (:Update
        (Transformation|SetRelativeLocation (Variables|Default|GetSwitch) (Math|Vector|MakeVector 0.0 0.0 _newtrack_0) false false)))))

(event OnComponentEndOverlap(OverlaptDetection)
  (params (OverlappedComponent :type Primitive%20Component%20Object%20Reference) (OtherActor :type Actor%20Object%20Reference) (OtherComp :type Primitive%20Component%20Object%20Reference) (OtherBodyIndex :type Integer))
  (if (Utilities|Array|IsEmpty (Collision|GetOverlappingActors (Variables|Default|GetOverlaptDetection) 0 :!class /Script/Engine.PrimitiveComponent))
    (Variables|Default|SetisActive false)
    (Variables|/Game/BluePrints/BoilerRoom/BP_FurnaceCable.BP_FurnaceCable_C|SetisFilling (Variables|Default|GetCableRef) true)
    (bind _newtrack_0 (Timeline|PressureMove Reverse)
      (:Update
        (Transformation|SetRelativeLocation (Variables|Default|GetSwitch) (Math|Vector|MakeVector 0.0 0.0 _newtrack_0) false false)))))

(fn ConstructionScript)