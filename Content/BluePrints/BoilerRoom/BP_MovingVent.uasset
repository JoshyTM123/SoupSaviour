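; BP_MovingVent is a boiler room fan vent that pushes cold-resistant players and physics objects along its up vector.
; Box overlaps track targets, and Tick applies launch or impulse force that weakens with height above the vent.
; Characters lacking cold resistance get a "too cold" widget instead of lift.
; An optional looping timer toggles force and wind effect, while MoveObject drives the vent along a referenced spline via timeline.
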(event OnComponentBeginOverlap(Box)
  (params (OverlappedComponent :type Primitive%20Component%20Object%20Reference) (OtherActor :type Actor%20Object%20Reference) (OtherComp :type Primitive%20Component%20Object%20Reference) (OtherBodyIndex :type Integer) (bFromSweep :type Boolean) (SweepResult :type Hit%20Result%20Structure%20%28by%20ref%29))
  (bind _overlappingactors (Variables|Default|GetOverlappingActors))
  ;[0.15 0.15 0.15 0.5] Adds and removes valid actors from an array of overlapped objects
  (bind _output_get (Variables|Default|SetOther%20Actor OtherActor))
  (bind _asbp_third_person_character (Utilities|Casting|CastToBP_ThirdPersonCharacter _output_get)
    (:then
      (Utilities|Array|AddUnique _overlappingactors (Variables|Default|GetOther%20Actor))
      (if (not (Variables|/Game/ThirdPerson/Blueprints/BP_ThirdPersonCharacter.BP_ThirdPersonCharacter_C|GetcoldResistant _asbp_third_person_character))
        (UserInterface|Viewport|AddtoViewport (Variables|Default|GetW_Cold) 0)))
    (:CastFailed
      (if (Physics|IsSimulatingPhysics (Variables|/Script/Engine.Actor|GetRootComponent OtherActor) "None")
        (Utilities|Array|AddUnique _overlappingactors (Variables|Default|GetOther%20Actor))))))

(event OnComponentEndOverlap(Box)
  (params (OverlappedComponent :type Primitive%20Component%20Object%20Reference) (OtherActor :type Actor%20Object%20Reference) (OtherComp :type Primitive%20Component%20Object%20Reference) (OtherBodyIndex :type Integer))
  ;[0.15 0.15 0.15 0.5] Adds and removes valid actors from an array of overlapped objects
  (if (Utilities|Array|ContainsItem (Variables|Default|GetOverlappingActors) OtherActor)
    (Utilities|Array|RemoveItem (Variables|Default|GetOverlappingActors) OtherActor)
    (if (UserInterface|Viewport|IsinViewport (Variables|Default|GetW_Cold))
      (Widget|RemovefromParent (Variables|Default|GetW_Cold)))))

(event Custom|Move%20Object
  (bind _splineref (Variables|Default|GetsplineRef))
  (bind _timedelay (Variables|Default|GettimeDelay))
  (bind _spline (Variables|/Game/BluePrints/BoilerRoom/BP_SplinePath.BP_SplinePath_C|GetSpline _splineref))
  (Rendering|Material|SetMaterial (Variables|Default|GetVent) 0 "/Game/CustomMaterials/PurpleGlow.PurpleGlow")
  (Utilities|FlowControl|Delay (Variables|Default|GettimeDelay))
  (Components|Timeline|SetPlayRate (Variables|Default|GetT_Move) (/ 1.0 (Variables|Default|GettimeToComplete)))
  (bind _move_track (Timeline|T_Move Play)
    (:Update
      (Transformation|SetActorLocation (Spline|GetLocationatDistanceAlongSpline _spline (Math|Float|Lerp 0.0 (Spline|GetSplineLength _spline) _move_track) "World") false false))
    (:Finished
      (if (Variables|Default|GetisMovingForward)
        (Utilities|FlowControl|Delay _timedelay)
        (Transformation|SetActorLocation "0, 0, 0" false false)
        (Utilities|String|Reverse (Variables|Default|GetT_Move))
        (Variables|Default|SetisMovingForward false)
        (else
          (Utilities|FlowControl|Delay _timedelay)
          (Transformation|SetActorLocation "0, 0, 0" false false)
          (Audio|Components|Audio|Play (Variables|Default|GetT_Move))
          (Variables|Default|SetisMovingForward true))))))

(event Custom|ToggleVent
  (Utilities|Time|SetTimerbyEvent (delegate Custom|FanOn/Off) (Variables|Default|GetOnOffTimer) true))

(event Custom|FanOn/Off
  (bind _windeffect (Variables|Default|GetWindEffect))
  ;[0.15 0.15 0.15 0.5] Turns vent off/on
  (Utilities|FlowControl|FlipFlop
    (:A
      (Rendering|SetVisibility _windeffect true false)
      (Variables|Default|SetisON true))
    (:B
      (Rendering|SetVisibility _windeffect false false)
      (Variables|Default|SetisON false))))

(event EventTick
  (params (DeltaSeconds :type Float%20%28single-precision%29))
  (bind _overlappingactors (Variables|Default|GetOverlappingActors))
  ;[0.15 0.15 0.15 0.5] Adds force to overlapped objects
  (if (Variables|Default|GetisON)
    (if (not (Utilities|Array|IsEmpty _overlappingactors))
      (for _array_element _overlappingactors
        (bind _asbp_third_person_character (Utilities|Casting|CastToBP_ThirdPersonCharacter _array_element)
          (:then
            (if (Variables|/Game/ThirdPerson/Blueprints/BP_ThirdPersonCharacter.BP_ThirdPersonCharacter_C|GetcoldResistant _asbp_third_person_character)
              (bind _baseforce (CallFunction|GetForceAmount true _array_element))
              (Character|LaunchCharacter _asbp_third_person_character _baseforce false false)))
          (:CastFailed
            (bind _asprimitive_component (Utilities|Casting|CastToPrimitiveComponent (Variables|/Script/Engine.Actor|GetRootComponent _array_element)))
            (bind _baseforce_2 (CallFunction|GetForceAmount false _array_element))
            (Class|PrimitiveComponent|AddVelocityChangeImpulseatLocation _asprimitive_component _baseforce_2 (Transformation|GetActorLocation _array_element) "None")))))))

(event EventBeginPlay
  (bind _windeffect (Variables|Default|GetWindEffect))
  ;[0.15 0.15 0.15 0.5] Gets max height of vent and turns particle system on/off
  (Variables|Default|SetMaxHeight (* (.z (Components|Box|GetScaledBoxExtent (Variables|Default|GetBox))) 2.0))
  (if (Variables|Default|GetisON)
    (Rendering|SetVisibility _windeffect true false)
    (else
      (Rendering|SetVisibility _windeffect false false)))
  (bind _returnvalue (UserInterface|CreateWidget "/Game/Widgets/W_TooCold.W_TooCold_C"))
  (Variables|Default|SetW_Cold _returnvalue)
  (if (Variables|Default|GetswitchesOnAndOff)
    (CallFunction|ToggleVent)))

(fn ConstructionScript)

(fn GetForceAmount
  (params (isCharacter :type Boolean) (CurrentActor :type Actor%20Object%20Reference))
  (if isCharacter
    (LocalVariables|SetForce (Variables|Default|GetPlayerForce))
    (else
      (LocalVariables|SetForce (Variables|Default|GetActorForce))))
  (return (* (- 1.0 (Math|Float|Clamp(Float) (/ (- (.z (Transformation|GetActorLocation CurrentActor)) (.z (Transformation|GetActorLocation))) (Variables|Default|GetMaxHeight)))) (Transformation|GetActorUpVector) (LocalVariables|GetForce))))