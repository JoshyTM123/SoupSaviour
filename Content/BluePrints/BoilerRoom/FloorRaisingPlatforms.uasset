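; Boiler room platform that, after TurnOn and an initial delay, cycles vertically up and down with pauses between moves.
; A timeline Z offset moves the actor from a stored start location, playing to rise and reversing to descend.
; On each finish, a FlipFlop alternates direction and recomputes the start location, using a hardcoded 500-unit drop before descending.
; The mesh material switches to purple glow while moving and silver while waiting.
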(event Custom|Up
  (bind _returnvalue (Transformation|GetActorLocation))
  (Rendering|Material|SetMaterial (Variables|Debug|GetStaticMeshComponent) 0 "/Game/CustomMaterials/PurpleGlow.PurpleGlow")
  (bind _z_offset (Timeline|T_Move Play)
    (:Update
      (Transformation|SetActorLocation (Math|Vector|MakeVector (.x (Variables|Default|GetStartLocation)) (.y (Variables|Default|GetStartLocation)) (+ _z_offset (.z (Variables|Default|GetStartLocation)))) false false))
    (:Finished
      (Rendering|Material|SetMaterial (Variables|Debug|GetStaticMeshComponent) 0 "/Game/CustomMaterials/Silver.Silver")
      (Utilities|FlowControl|Delay (Variables|Default|GetDelay))
      (Utilities|FlowControl|FlipFlop
        (:A
          (Variables|Default|SetStartLocation (Math|Vector|MakeVector (.x _returnvalue) (.y _returnvalue) (- (.z _returnvalue) 5e+02)))
          (CallFunction|Down))
        (:B
          (Variables|Default|SetStartLocation (Transformation|GetActorLocation))
          (CallFunction|Up))))))

(event Custom|Down
  (bind _returnvalue (Transformation|GetActorLocation))
  (Rendering|Material|SetMaterial (Variables|Debug|GetStaticMeshComponent) 0 "/Game/CustomMaterials/PurpleGlow.PurpleGlow")
  (bind _z_offset (Timeline|T_Move Reverse)
    (:Update
      (Transformation|SetActorLocation (Math|Vector|MakeVector (.x (Variables|Default|GetStartLocation)) (.y (Variables|Default|GetStartLocation)) (+ _z_offset (.z (Variables|Default|GetStartLocation)))) false false))
    (:Finished
      (Rendering|Material|SetMaterial (Variables|Debug|GetStaticMeshComponent) 0 "/Game/CustomMaterials/Silver.Silver")
      (Utilities|FlowControl|Delay (Variables|Default|GetDelay))
      (Utilities|FlowControl|FlipFlop
        (:A
          (Variables|Default|SetStartLocation (Math|Vector|MakeVector (.x _returnvalue) (.y _returnvalue) (- (.z _returnvalue) 5e+02)))
          (CallFunction|Down))
        (:B
          (Variables|Default|SetStartLocation (Transformation|GetActorLocation))
          (CallFunction|Up))))))

(event Custom|TurnOn
  (Utilities|FlowControl|Delay (Variables|Default|GetinitialDelay))
  (Variables|Default|SetStartLocation (Transformation|GetActorLocation))
  (CallFunction|Up))

(fn ConstructionScript)