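; BP_PlatformPP is a pressure plate in the boiler room that drives a referenced platform and can itself slide along Y.
; Its GoForwards and GoBackwards events play or reverse the slide timeline after a delay.
; The first overlap lowers or raises the switch via a timeline and sends PlatformRef forwards; emptying the trigger reverses both.
; With IncludePP set, the linked PP receives GoForwards on both press and release, never GoBackwards.
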(event OnComponentBeginOverlap(OverlaptDetection)
  (params (OverlappedComponent :type Primitive%20Component%20Object%20Reference) (OtherActor :type Actor%20Object%20Reference) (OtherComp :type Primitive%20Component%20Object%20Reference) (OtherBodyIndex :type Integer) (bFromSweep :type Boolean) (SweepResult :type Hit%20Result%20Structure%20%28by%20ref%29))
  (if (not (Variables|Default|GetisActive))
    (Variables|Default|SetisActive true)
    (Default|GoForwards (Variables|Default|GetplatformRef))
    (if (Variables|Default|GetincludePP)
      (CallFunction|GoForwards (Variables|Default|GetPP))
      (bind _newtrack_0 (Timeline|PressureMove Play)
        (:Update
          (Transformation|SetRelativeLocation (Variables|Default|GetSwitch) (Math|Vector|MakeVector 0.0 0.0 _newtrack_0) false false)))
      (else
        (Timeline|PressureMove Play)))))

(event OnComponentEndOverlap(OverlaptDetection)
  (params (OverlappedComponent :type Primitive%20Component%20Object%20Reference) (OtherActor :type Actor%20Object%20Reference) (OtherComp :type Primitive%20Component%20Object%20Reference) (OtherBodyIndex :type Integer))
  (if (Utilities|Array|IsEmpty (Collision|GetOverlappingActors (Variables|Default|GetOverlaptDetection) 0 :!class /Script/Engine.PrimitiveComponent))
    (Variables|Default|SetisActive false)
    (Default|GoBackwards (Variables|Default|GetplatformRef))
    (if (Variables|Default|GetincludePP)
      (CallFunction|GoForwards (Variables|Default|GetPP))
      (bind _newtrack_0 (Timeline|PressureMove Reverse)
        (:Update
          (Transformation|SetRelativeLocation (Variables|Default|GetSwitch) (Math|Vector|MakeVector 0.0 0.0 _newtrack_0) false false)))
      (else
        (Timeline|PressureMove Reverse)))))

(event Custom|GoBackwards
  (Utilities|FlowControl|Delay (Variables|Default|GetDelayTime))
  (bind _position (Timeline|Timeline Reverse)
    (:Update
      (Transformation|SetRelativeLocation (Variables|Default|GetDefaultSceneRoot) (Math|Vector|MakeVector 0.0 _position 0.0) false false))))

(event Custom|GoForwards
  (Utilities|FlowControl|Delay (Variables|Default|GetDelayTime))
  (bind _position (Timeline|Timeline Play)
    (:Update
      (Transformation|SetRelativeLocation (Variables|Default|GetDefaultSceneRoot) (Math|Vector|MakeVector 0.0 _position 0.0) false false))))

(fn ConstructionScript)