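; BP_Cage is a cage with a door that opens while a required number of switches are active.
; SwitchActivated and SwitchDeactivated adjust a counter and compare it to SwitchesNeeded.
; A timeline moves the door along relative Z, playing forward to open and reversing to close.
; Zap and lift sounds play whenever the threshold check passes, while the close sound plays only if the door was open.
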(event Custom|SwitchActivated
  (bind _returnvalue (Transformation|GetActorLocation))
  ;[0.15 0.15 0.15 0.5] Will either open or close door by moving its z axis up/down
  (Math|Integer|IncrementInt (Variables|Default|GetSwitchesActivated)
    (:%20%20
      (if (>= (Variables|Default|GetSwitchesActivated) (Variables|Default|GetSwitchesNeeded))
        ;;[0.15 0.15 0.15 0.5] Open Door
        (Audio|PlaySoundatLocation "/Game/Audio/Electric_Zap.Electric_Zap" _returnvalue "0, 0, 0" 1.0 1.0 0.0 0 0 0 0)
        (Audio|PlaySoundatLocation "/Game/Audio/metal_door_lift.metal_door_lift" _returnvalue "0, 0, 0" 0.5 1.0 0.0 0 0 0 0)
        (Variables|Default|SetisOpen true)
        (bind _doorposition (Timeline|Timeline Play)
          (:Update
            (Transformation|SetRelativeLocation (Variables|Default|GetDoor) (Math|Vector|MakeVector 0.0 0.0 _doorposition) false false)))
        (elif (Variables|Default|GetisOpen)
          ;;[0.15 0.15 0.15 0.5] Close Door
          (Audio|PlaySoundatLocation "/Game/Audio/metal_door_close.metal_door_close" (Transformation|GetActorLocation) "0, 0, 0" 0.5 1.0 0.0 0 0 0 0)
          (Variables|Default|SetisOpen false)
          (Timeline|Timeline Reverse)
          (else
            (Timeline|Timeline Reverse)))))))

(event Custom|SwitchDeactivated
  (bind _returnvalue (Transformation|GetActorLocation))
  ;[0.15 0.15 0.15 0.5] Will either open or close door by moving its z axis up/down
  (Math|Integer|DecrementInt (Variables|Default|GetSwitchesActivated)
    (:%20%20
      (if (>= (Variables|Default|GetSwitchesActivated) (Variables|Default|GetSwitchesNeeded))
        ;;[0.15 0.15 0.15 0.5] Open Door
        (Audio|PlaySoundatLocation "/Game/Audio/Electric_Zap.Electric_Zap" _returnvalue "0, 0, 0" 1.0 1.0 0.0 0 0 0 0)
        (Audio|PlaySoundatLocation "/Game/Audio/metal_door_lift.metal_door_lift" _returnvalue "0, 0, 0" 0.5 1.0 0.0 0 0 0 0)
        (Variables|Default|SetisOpen true)
        (bind _doorposition (Timeline|Timeline Play)
          (:Update
            (Transformation|SetRelativeLocation (Variables|Default|GetDoor) (Math|Vector|MakeVector 0.0 0.0 _doorposition) false false)))
        (elif (Variables|Default|GetisOpen)
          ;;[0.15 0.15 0.15 0.5] Close Door
          (Audio|PlaySoundatLocation "/Game/Audio/metal_door_close.metal_door_close" (Transformation|GetActorLocation) "0, 0, 0" 0.5 1.0 0.0 0 0 0 0)
          (Variables|Default|SetisOpen false)
          (Timeline|Timeline Reverse)
          (else
            (Timeline|Timeline Reverse)))))))

(fn ConstructionScript)