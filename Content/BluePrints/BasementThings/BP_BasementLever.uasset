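; BP_BasementLever is an interactable basement lever that switches filling on and off on a referenced cable.
; Each Interact call flip-flops the cable's IsFilling flag, rotates the lever and plays a switch sound, adding a positional electric zap when switched on.
; A box trigger shows and hides a W_Interact prompt, created at BeginPlay, as the player character enters and leaves.
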(event OnComponentBeginOverlap(Box)
  (params (OverlappedComponent :type Primitive%20Component%20Object%20Reference) (OtherActor :type Actor%20Object%20Reference) (OtherComp :type Primitive%20Component%20Object%20Reference) (OtherBodyIndex :type Integer) (bFromSweep :type Boolean) (SweepResult :type Hit%20Result%20Structure%20%28by%20ref%29))
  ;[0.15 0.15 0.15 0.5] Display Widget
  (if (== OtherActor (Game|GetPlayerCharacter 0))
    (UserInterface|Viewport|AddtoViewport (Variables|Default|GetIP) 0)))

(event OnComponentEndOverlap(Box)
  (params (OverlappedComponent :type Primitive%20Component%20Object%20Reference) (OtherActor :type Actor%20Object%20Reference) (OtherComp :type Primitive%20Component%20Object%20Reference) (OtherBodyIndex :type Integer))
  ;[0.15 0.15 0.15 0.5] Display Widget
  (if (== (Game|GetPlayerCharacter 0) OtherActor)
    (Widget|RemovefromParent (Variables|Default|GetIP))))

(event EventBeginPlay
  ;[0.15 0.15 0.15 0.5] Display Widget
  (bind _returnvalue (UserInterface|CreateWidget "/Game/Widgets/W_Interact.W_Interact_C"))
  (bind _output_get (Variables|Default|SetIP _returnvalue))
  (Variables|/Game/Widgets/W_Interact.W_Interact_C|SetPromptText _output_get "Press 'E' to pull lever"))

(event EventInteract
  (bind _cableref (Variables|Default|GetCableRef))
  (Utilities|FlowControl|FlipFlop
    (:A
      (Variables|/Game/BluePrints/BasementThings/BP_Cable.BP_Cable_C|SetisFilling _cableref true)
      (Audio|PlaySoundatLocation "/Game/Audio/Electric_Zap.Electric_Zap" (Transformation|GetWorldLocation (Variables|Default|GetLeverBase)) "0, 0, 0" 1.0 1.0 0.0 0 0 0 0)
      (Audio|PlaySound2D "/Game/Audio/SwitchOn.SwitchOn" 1.0 1.0 0.0 0 0)
      (Transformation|SetRelativeRotation (Variables|Default|GetLever) "0.000000,0.000000,110.000000" false false))
    (:B
      (Variables|/Game/BluePrints/BasementThings/BP_Cable.BP_Cable_C|SetisFilling _cableref false)
      (Audio|PlaySound2D "/Game/Audio/switchOff.switchOff" 1.0 1.0 0.0 0 0)
      (Transformation|SetRelativeRotation (Variables|Default|GetLever) "0.000000,0.000000,70.000000" false false))))

(fn ConstructionScript)

(fn ReturnText
  (return ""))