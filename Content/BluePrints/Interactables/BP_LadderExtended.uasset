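; BP_LadderExtended is an interactable ladder that the third-person character can climb once it has been extended.
; Interact sets the root component's scale to triple size on all axes and flags the ladder as extended.
; While that flag is set, the Box overlap begin and end events turn climbing on and off through the character's OnClimbing.
; ReturnText returns an empty string.
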(event OnComponentBeginOverlap(Box)
  (params (OverlappedComponent :type Primitive%20Component%20Object%20Reference) (OtherActor :type Actor%20Object%20Reference) (OtherComp :type Primitive%20Component%20Object%20Reference) (OtherBodyIndex :type Integer) (bFromSweep :type Boolean) (SweepResult :type Hit%20Result%20Structure%20%28by%20ref%29))
  ;[0.15 0.15 0.15 0.5] Only climbable if ladder has been extended
  (if (Variables|Default|GetisExtended)
    (bind _asbp_third_person_character (Utilities|Casting|CastToBP_ThirdPersonCharacter OtherActor))
    (Default|OnClimbing _asbp_third_person_character true)))

(event OnComponentEndOverlap(Box)
  (params (OverlappedComponent :type Primitive%20Component%20Object%20Reference) (OtherActor :type Actor%20Object%20Reference) (OtherComp :type Primitive%20Component%20Object%20Reference) (OtherBodyIndex :type Integer))
  ;[0.15 0.15 0.15 0.5] Only climbable if ladder has been extended
  (if (Variables|Default|GetisExtended)
    (bind _asbp_third_person_character (Utilities|Casting|CastToBP_ThirdPersonCharacter OtherActor))
    (Default|OnClimbing _asbp_third_person_character false)))

(event EventInteract
  (Transformation|SetRelativeScale3D (Variables|Default|GetDefaultSceneRoot) "3.000000,3.000000,3.000000")
  (Variables|Default|SetisExtended true))

(fn ConstructionScript)

(fn ReturnText
  (return ""))