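; Breakable wall interactable that the player destroys while holding the sledgehammer.
; Interact checks the character's ItemHeld enum, destroying the wall on a match or printing a debug message otherwise.
; A Box overlap shows a W_Interact widget, created at BeginPlay, with prompt text matching the held item, and removes it when the player leaves.
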(event OnComponentBeginOverlap(Box)
  (params (OverlappedComponent :type Primitive%20Component%20Object%20Reference) (OtherActor :type Actor%20Object%20Reference) (OtherComp :type Primitive%20Component%20Object%20Reference) (OtherBodyIndex :type Integer) (bFromSweep :type Boolean) (SweepResult :type Hit%20Result%20Structure%20%28by%20ref%29))
  (bind _ip (Variables|Default|GetIP))
  ;[0.15 0.15 0.15 0.5] Display Widget
  (if (== OtherActor (Game|GetPlayerCharacter 0))
    (bind _asbp_third_person_character (Utilities|Casting|CastToBP_ThirdPersonCharacter (Game|GetPlayerCharacter 0)))
    (if (Utilities|Enum|Equal(Enum) (Variables|/Game/ThirdPerson/Blueprints/BP_ThirdPersonCharacter.BP_ThirdPersonCharacter_C|GetItemHeld _asbp_third_person_character) "NewEnumerator1")
      (Variables|/Game/Widgets/W_Interact.W_Interact_C|SetPromptText _ip "Press 'E' to break wall")
      (else
        (Variables|/Game/Widgets/W_Interact.W_Interact_C|SetPromptText _ip "Need Sledgehammer to interact")))
    (UserInterface|Viewport|AddtoViewport _ip 0)))

(event OnComponentEndOverlap(Box)
  (params (OverlappedComponent :type Primitive%20Component%20Object%20Reference) (OtherActor :type Actor%20Object%20Reference) (OtherComp :type Primitive%20Component%20Object%20Reference) (OtherBodyIndex :type Integer))
  ;[0.15 0.15 0.15 0.5] Display Widget
  (if (== (Game|GetPlayerCharacter 0) OtherActor)
    (Widget|RemovefromParent (Variables|Default|GetIP))))

(event EventBeginPlay
  ;[0.15 0.15 0.15 0.5] Display Widget
  (bind _returnvalue (UserInterface|CreateWidget "/Game/Widgets/W_Interact.W_Interact_C"))
  (Variables|Default|SetIP _returnvalue))

(event EventInteract
  (bind _asbp_third_person_character (Utilities|Casting|CastToBP_ThirdPersonCharacter (Game|GetPlayerCharacter 0)))
  (if (Utilities|Enum|Equal(Enum) (Variables|/Game/ThirdPerson/Blueprints/BP_ThirdPersonCharacter.BP_ThirdPersonCharacter_C|GetItemHeld _asbp_third_person_character) "NewEnumerator1")
    (Actor|DestroyActor)
    (else
      (Development|PrintString "NOT HOLDING SLEDGEHAMMER"))))

(fn ConstructionScript)

(fn ReturnText
  (return ""))