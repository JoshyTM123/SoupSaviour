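; BP_Cube is an interactable cube that shows a pickup prompt when the player comes near.
; It creates an interact widget on BeginPlay and adds or removes it as the player character enters or leaves its Box trigger.
; On entry it reads the character's PickupUnlocked flag to show either a left-click pickup hint or a strength-required message.
; The Blueprint handles only the prompt, with no pickup logic of its own.
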(event OnComponentBeginOverlap(Box)
  (params (OverlappedComponent :type Primitive%20Component%20Object%20Reference) (OtherActor :type Actor%20Object%20Reference) (OtherComp :type Primitive%20Component%20Object%20Reference) (OtherBodyIndex :type Integer) (bFromSweep :type Boolean) (SweepResult :type Hit%20Result%20Structure%20%28by%20ref%29))
  (bind _w_prompt (Variables|Default|GetW_Prompt))
  ;[0.15 0.15 0.15 0.5] Display Widget
  (if (== OtherActor (Game|GetPlayerCharacter 0))
    (bind _asbp_third_person_character (Utilities|Casting|CastToBP_ThirdPersonCharacter (Game|GetPlayerCharacter 0)))
    (if (Variables|/Game/ThirdPerson/Blueprints/BP_ThirdPersonCharacter.BP_ThirdPersonCharacter_C|GetpickupUnlocked _asbp_third_person_character)
      (Variables|/Game/Widgets/W_Interact.W_Interact_C|SetPromptText _w_prompt "Left click to pickup object")
      (else
        (Variables|/Game/Widgets/W_Interact.W_Interact_C|SetPromptText _w_prompt "Strength required to pickup")))
    (UserInterface|Viewport|AddtoViewport _w_prompt 0)))

(event OnComponentEndOverlap(Box)
  (params (OverlappedComponent :type Primitive%20Component%20Object%20Reference) (OtherActor :type Actor%20Object%20Reference) (OtherComp :type Primitive%20Component%20Object%20Reference) (OtherBodyIndex :type Integer))
  ;[0.15 0.15 0.15 0.5] Display Widget
  (if (== (Game|GetPlayerCharacter 0) OtherActor)
    (Widget|RemovefromParent (Variables|Default|GetW_Prompt))))

(event EventBeginPlay
  ;[0.15 0.15 0.15 0.5] Display Widget
  (bind _returnvalue (UserInterface|CreateWidget "/Game/Widgets/W_Interact.W_Interact_C"))
  (Variables|Default|SetW_Prompt _returnvalue))

(fn ConstructionScript)