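; BP_Plank is an interactable plank that the player breaks while holding the sledgehammer.
; A box overlap shows a W_Interact prompt that depends on the character's held item and removes it on exit.
; Interact plays a hit sound, swaps visibility and collision from the Pos1 actor to Pos2, then destroys the plank.
; BeginPlay creates the widget and disables only Pos2's collision, leaving its visibility untouched.
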(event OnComponentBeginOverlap(Box)
  (params (OverlappedComponent :type Primitive%20Component%20Object%20Reference) (OtherActor :type Actor%20Object%20Reference) (OtherComp :type Primitive%20Component%20Object%20Reference) (OtherBodyIndex :type Integer) (bFromSweep :type Boolean) (SweepResult :type Hit%20Result%20Structure%20%28by%20ref%29))
  (bind _interactw (Variables|Default|GetInteractW))
  ;[0.15 0.15 0.15 0.5] Display Widget
  (if (== OtherActor (Game|GetPlayerCharacter 0))
    (bind _asbp_third_person_character (Utilities|Casting|CastToBP_ThirdPersonCharacter (Game|GetPlayerCharacter 0)))
    (if (Utilities|Enum|Equal(Enum) (Variables|/Game/ThirdPerson/Blueprints/BP_ThirdPersonCharacter.BP_ThirdPersonCharacter_C|GetItemHeld _asbp_third_person_character) "NewEnumerator1")
      (Variables|/Game/Widgets/W_Interact.W_Interact_C|SetPromptText _interactw "Press 'E' to break plank")
      (else
        (Variables|/Game/Widgets/W_Interact.W_Interact_C|SetPromptText _interactw "Need Sledgehammer")))
    (UserInterface|Viewport|AddtoViewport _interactw 0)))

(event OnComponentEndOverlap(Box)
  (params (OverlappedComponent :type Primitive%20Component%20Object%20Reference) (OtherActor :type Actor%20Object%20Reference) (OtherComp :type Primitive%20Component%20Object%20Reference) (OtherBodyIndex :type Integer))
  ;[0.15 0.15 0.15 0.5] Display Widget
  (if (== (Game|GetPlayerCharacter 0) OtherActor)
    (Widget|RemovefromParent (Variables|Default|GetInteractW))))

(event EventInteract
  (bind _pos2 (Variables|Default|Getpos2))
  (bind _pos1 (Variables|Default|Getpos1))
  ;[0.15 0.15 0.15 0.5] Interact
  (bind _asbp_third_person_character (Utilities|Casting|CastToBP_ThirdPersonCharacter (Game|GetPlayerCharacter 0)))
  (if (Utilities|Enum|Equal(Enum) (Variables|/Game/ThirdPerson/Blueprints/BP_ThirdPersonCharacter.BP_ThirdPersonCharacter_C|GetItemHeld _asbp_third_person_character) "NewEnumerator1")
    (Audio|PlaySound2D "/Game/Audio/HammerHit.HammerHit" 1.0 1.0 0.0 0 0)
    (Rendering|SetActorHiddenInGame _pos1 true)
    (Collision|SetActorEnableCollision _pos1 false)
    (Rendering|SetActorHiddenInGame _pos2 false)
    (Collision|SetActorEnableCollision _pos2 true)
    (Actor|DestroyActor)))

(event EventBeginPlay
  ;[0.15 0.15 0.15 0.5] Hide second plank at start
  (Collision|SetActorEnableCollision (Variables|Default|Getpos2) false)
  (bind _returnvalue (UserInterface|CreateWidget "/Game/Widgets/W_Interact.W_Interact_C"))
  (Variables|Default|SetInteractW _returnvalue))

(fn ConstructionScript)

(fn ReturnText
  (return ""))