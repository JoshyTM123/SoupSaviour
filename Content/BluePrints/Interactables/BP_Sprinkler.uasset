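; BP_Sprinkler is a one-time interactable that turns on a sprinkler to grow plants, with water effects and a cutscene.
; A box overlap shows or hides the "Press 'E'" prompt widget for the player.
; Interact activates each plant pot and, within that same loop, spawns Niagara droplets at hardcoded world locations and plays the level sequence.
; Player input is disabled for the sequence's duration, then restored as HasPlayed blocks reuse.
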(event OnComponentBeginOverlap(Box)
  (params (OverlappedComponent :type Primitive%20Component%20Object%20Reference) (OtherActor :type Actor%20Object%20Reference) (OtherComp :type Primitive%20Component%20Object%20Reference) (OtherBodyIndex :type Integer) (bFromSweep :type Boolean) (SweepResult :type Hit%20Result%20Structure%20%28by%20ref%29))
  ;[0.15 0.15 0.15 0.5] Display Widget (Interactable)
  (if (== OtherActor (Game|GetPlayerCharacter 0))
    (if (not (Variables|Default|GethasPlayed))
      (UserInterface|Viewport|AddtoViewport (Variables|Default|Getw_interact) 0))))

(event OnComponentEndOverlap(Box)
  (params (OverlappedComponent :type Primitive%20Component%20Object%20Reference) (OtherActor :type Actor%20Object%20Reference) (OtherComp :type Primitive%20Component%20Object%20Reference) (OtherBodyIndex :type Integer))
  ;[0.15 0.15 0.15 0.5] Display Widget (Interactable)
  (if (== (Game|GetPlayerCharacter 0) OtherActor)
    (Widget|RemovefromParent (Variables|Default|Getw_interact))))

(event EventBeginPlay
  ;[0.15 0.15 0.15 0.5] Display Widget (Interactable)
  (bind _returnvalue (UserInterface|CreateWidget "/Game/Widgets/W_Interact.W_Interact_C"))
  (bind _output_get (Variables|Default|Setw_interact _returnvalue))
  (Variables|/Game/Widgets/W_Interact.W_Interact_C|SetPromptText _output_get "Press 'E' to turn on sprinkler"))

(event EventInteract
  (bind _levsequenceref (Variables|Default|GetLevSequenceRef))
  (bind _sequenceplayer (Variables|/Script/LevelSequence.LevelSequenceActor|GetSequencePlayer _levsequenceref))
  ;[0.15 0.15 0.15 0.5] Play cutscene, spawn plants and water droplets
  (if (not (Variables|Default|GethasPlayed))
    (for _array_element (Variables|Default|GetPlantPots)
      (Default|Activate _array_element)
      (Niagara|SpawnSystematLocation "/Game/CustomMaterials/CustomNS/NS_WaterDrop.NS_WaterDrop" "5215.098608,1438.862821,2000.000000")
      (Niagara|SpawnSystematLocation "/Game/CustomMaterials/CustomNS/NS_WaterDrop.NS_WaterDrop" "5328.511171,2325.555306,2000.000000")
      (Niagara|SpawnSystematLocation "/Game/CustomMaterials/CustomNS/NS_WaterDrop.NS_WaterDrop" "5340.295053,3830.198260,2000.000000")
      (bind _asbp_third_person_character (Utilities|Casting|CastToBP_ThirdPersonCharacter (Game|GetPlayerCharacter 0)))
      (Input|DisableInput _asbp_third_person_character 0)
      (Sequencer|Player|Play _sequenceplayer :!class /Script/MovieScene.MovieSceneSequencePlayer)
      (Utilities|FlowControl|Delay (Class|TimeManagementBlueprintLibrary|ToSeconds(QualifiedFrameTime) (Media|MediaPlayer|GetDuration _sequenceplayer)))
      (Input|EnableInput _asbp_third_person_character 0)
      (Variables|Default|SethasPlayed true))))

(fn ConstructionScript)

(fn ReturnText
  (return ""))