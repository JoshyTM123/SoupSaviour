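; BP_Steak is an interactable steak pickup that the player can eat.
; A box overlap with the player shows and hides a W_Interact prompt widget created on BeginPlay.
; Interact sets PickupUnlocked on the player character, registers "Steak" through the game instance's UpdateIngredients, then destroys the actor.
; ReturnText supplies the same prompt string.
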(event OnComponentBeginOverlap(Box)
  (params (OverlappedComponent :type Primitive%20Component%20Object%20Reference) (OtherActor :type Actor%20Object%20Reference) (OtherComp :type Primitive%20Component%20Object%20Reference) (OtherBodyIndex :type Integer) (bFromSweep :type Boolean) (SweepResult :type Hit%20Result%20Structure%20%28by%20ref%29))
  ;[0.15 0.15 0.15 0.5] Display Widget
  (if (== OtherActor (Game|GetPlayerCharacter 0))
    (UserInterface|Viewport|AddtoViewport (Variables|Default|GetInteractPrompt) 0)))

(event OnComponentEndOverlap(Box)
  (params (OverlappedComponent :type Primitive%20Component%20Object%20Reference) (OtherActor :type Actor%20Object%20Reference) (OtherComp :type Primitive%20Component%20Object%20Reference) (OtherBodyIndex :type Integer))
  ;[0.15 0.15 0.15 0.5] Display Widget
  (if (== (Game|GetPlayerCharacter 0) OtherActor)
    (Widget|RemovefromParent (Variables|Default|GetInteractPrompt))))

(event EventBeginPlay
  ;[0.15 0.15 0.15 0.5] Display Widget
  (bind _returnvalue (UserInterface|CreateWidget "/Game/Widgets/W_Interact.W_Interact_C"))
  (bind _output_get (Variables|Default|SetInteractPrompt _returnvalue))
  (Variables|/Game/Widgets/W_Interact.W_Interact_C|SetPromptText _output_get "Press 'E' to eat steak"))

(event EventInteract
  (bind _asbp_third_person_character (Utilities|Casting|CastToBP_ThirdPersonCharacter (Game|GetPlayerCharacter 0)))
  (Variables|/Game/ThirdPerson/Blueprints/BP_ThirdPersonCharacter.BP_ThirdPersonCharacter_C|SetpickupUnlocked _asbp_third_person_character true)
  (bind _asbp_game_instance (Utilities|Casting|CastToBP_GameInstance (Game|GetGameInstance)))
  (Default|UpdateIngredients _asbp_game_instance "Steak")
  (Actor|DestroyActor))

(fn ConstructionScript)

(fn ReturnText
  (return "Press 'E' to eat steak"))