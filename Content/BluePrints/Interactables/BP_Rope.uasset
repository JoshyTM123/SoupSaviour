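; Interactable rope that the player extends to create a climbable route.
; Interact snaps the root component to an extended scale and location and marks the rope as extended.
; Once extended, overlapping the Box toggles climbing on BP_ThirdPersonCharacter.
; While unextended, a separate detector volume shows and hides a W_Interact prompt for the player, created on BeginPlay.
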(event OnComponentBeginOverlap(Box)
  (params (OverlappedComponent :type Primitive%20Component%20Object%20Reference) (OtherActor :type Actor%20Object%20Reference) (OtherComp :type Primitive%20Component%20Object%20Reference) (OtherBodyIndex :type Integer) (bFromSweep :type Boolean) (SweepResult :type Hit%20Result%20Structure%20%28by%20ref%29))
  ;[0.15 0.15 0.15 0.5] Set player climbing to true/false IF EXTENDED
  (if (Variables|Default|GetisExtended)
    (bind _asbp_third_person_character (Utilities|Casting|CastToBP_ThirdPersonCharacter OtherActor))
    (Default|OnClimbing _asbp_third_person_character true)))

(event OnComponentEndOverlap(Box)
  (params (OverlappedComponent :type Primitive%20Component%20Object%20Reference) (OtherActor :type Actor%20Object%20Reference) (OtherComp :type Primitive%20Component%20Object%20Reference) (OtherBodyIndex :type Integer))
  ;[0.15 0.15 0.15 0.5] Set player climbing to true/false IF EXTENDED
  (if (Variables|Default|GetisExtended)
    (bind _asbp_third_person_character (Utilities|Casting|CastToBP_ThirdPersonCharacter OtherActor))
    (Default|OnClimbing _asbp_third_person_character false)))

(event OnComponentBeginOverlap(WidgetTextDetector)
  (params (OverlappedComponent :type Primitive%20Component%20Object%20Reference) (OtherActor :type Actor%20Object%20Reference) (OtherComp :type Primitive%20Component%20Object%20Reference) (OtherBodyIndex :type Integer) (bFromSweep :type Boolean) (SweepResult :type Hit%20Result%20Structure%20%28by%20ref%29))
  ;[0.15 0.15 0.15 0.5] Display Widget
  (if (and (== OtherActor (Game|GetPlayerCharacter 0)) (not (Variables|Default|GetisExtended)))
    (UserInterface|Viewport|AddtoViewport (Variables|Default|GetInteractPrompt) 0)))

(event OnComponentEndOverlap(WidgetTextDetector)
  (params (OverlappedComponent :type Primitive%20Component%20Object%20Reference) (OtherActor :type Actor%20Object%20Reference) (OtherComp :type Primitive%20Component%20Object%20Reference) (OtherBodyIndex :type Integer))
  ;[0.15 0.15 0.15 0.5] Display Widget
  (if (and (== (Game|GetPlayerCharacter 0) OtherActor) (not (Variables|Default|GetisExtended)))
    (Widget|RemovefromParent (Variables|Default|GetInteractPrompt))))

(event EventBeginPlay
  ;[0.15 0.15 0.15 0.5] Display Widget
  (bind _returnvalue (UserInterface|CreateWidget "/Game/Widgets/W_Interact.W_Interact_C"))
  (bind _output_get (Variables|Default|SetInteractPrompt _returnvalue))
  (Variables|/Game/Widgets/W_Interact.W_Interact_C|SetPromptText _output_get "Press 'E' to extend rope"))

(event EventInteract
  ;[0.15 0.15 0.15 0.5] Extends Rope
  (Transformation|SetWorldScale3D (Variables|Default|GetDefaultSceneRoot) (Variables|Default|GetExtendedScale))
  (Transformation|SetWorldLocation (Variables|Default|GetDefaultSceneRoot) (Variables|Default|GetExtendedLocation) false true)
  (Variables|Default|SetisExtended true))

(fn ConstructionScript)

(fn ReturnText
  (return ""))