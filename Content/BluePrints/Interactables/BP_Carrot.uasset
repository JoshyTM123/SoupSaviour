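; BP_Carrot is an interactable carrot pickup that, when consumed, unlocks night vision on the player's BP_ThirdPersonCharacter and destroys itself.
; Interaction only works when it is not frozen; Unfreeze hides the ice block, drops its collision, enables carrot physics and swaps to a glowing orange material.
; A box overlap adds and removes a W_Interact prompt widget, created on BeginPlay, for the player.
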(event OnComponentBeginOverlap(Box)
  (params (OverlappedComponent :type Primitive%20Component%20Object%20Reference) (OtherActor :type Actor%20Object%20Reference) (OtherComp :type Primitive%20Component%20Object%20Reference) (OtherBodyIndex :type Integer) (bFromSweep :type Boolean) (SweepResult :type Hit%20Result%20Structure%20%28by%20ref%29))
  ;[0.15 0.15 0.15 0.5] Widget Shenanigans
  (if (== OtherActor (Game|GetPlayerCharacter 0))
    (UserInterface|Viewport|AddtoViewport (Variables|Default|GetInteractWidget) 0)))

(event OnComponentEndOverlap(Box)
  (params (OverlappedComponent :type Primitive%20Component%20Object%20Reference) (OtherActor :type Actor%20Object%20Reference) (OtherComp :type Primitive%20Component%20Object%20Reference) (OtherBodyIndex :type Integer))
  ;[0.15 0.15 0.15 0.5] Widget Shenanigans
  (if (== (Game|GetPlayerCharacter 0) OtherActor)
    (Widget|RemovefromParent (Variables|Default|GetInteractWidget))))

(event EventInteract
  (if (not (Variables|Default|GetisFrozen))
    (bind _asbp_third_person_character (Utilities|Casting|CastToBP_ThirdPersonCharacter (Game|GetPlayerCharacter 0)))
    (Variables|/Game/ThirdPerson/Blueprints/BP_ThirdPersonCharacter.BP_ThirdPersonCharacter_C|SetnightVisionUnlocked _asbp_third_person_character true)
    (Actor|DestroyActor)))

(event EventBeginPlay
  ;[0.15 0.15 0.15 0.5] Widget Shenanigans
  (bind _returnvalue (UserInterface|CreateWidget "/Game/Widgets/W_Interact.W_Interact_C"))
  (bind _output_get (Variables|Default|SetInteractWidget _returnvalue))
  (Variables|/Game/Widgets/W_Interact.W_Interact_C|SetPromptText _output_get "Press E to consume carrot"))

(fn ConstructionScript)

(fn Unfreeze
  (Rendering|SetVisibility (Variables|Default|GetIceBlock) false false)
  (Collision|SetCollisionEnabled (Variables|Default|GetIceBlock) "NoCollision")
  (Physics|SetSimulatePhysics (Variables|Default|GetCarrot) true)
  (Rendering|Material|SetMaterial (Variables|Default|GetCarrot) 0 "/Game/CustomMaterials/M_GlowingOrange.M_GlowingOrange")
  (Variables|Default|SetisFrozen false))

(fn ReturnText
  (return ""))