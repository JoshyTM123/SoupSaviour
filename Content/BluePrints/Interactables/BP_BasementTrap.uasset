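; BP_BasementTrap is an interactable basement hatch that destroys itself when Interact is called.
; On BeginPlay it creates a W_Interact widget with an "open hatch" prompt.
; Box overlap events show and hide that prompt for BP_ThirdPersonCharacter, only when NightVisionUnlocked is true.
; Interact itself does not check that unlock, and ReturnText returns an empty string.
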(event OnComponentBeginOverlap(Box)
  (params (OverlappedComponent :type Primitive%20Component%20Object%20Reference) (OtherActor :type Actor%20Object%20Reference) (OtherComp :type Primitive%20Component%20Object%20Reference) (OtherBodyIndex :type Integer) (bFromSweep :type Boolean) (SweepResult :type Hit%20Result%20Structure%20%28by%20ref%29))
  ;[0.15 0.15 0.15 0.5] Display Widget
  (bind _asbp_third_person_character (Utilities|Casting|CastToBP_ThirdPersonCharacter OtherActor))
  (if (Variables|/Game/ThirdPerson/Blueprints/BP_ThirdPersonCharacter.BP_ThirdPersonCharacter_C|GetnightVisionUnlocked _asbp_third_person_character)
    (UserInterface|Viewport|AddtoViewport (Variables|Default|GetNewVar) 0)))

(event OnComponentEndOverlap(Box)
  (params (OverlappedComponent :type Primitive%20Component%20Object%20Reference) (OtherActor :type Actor%20Object%20Reference) (OtherComp :type Primitive%20Component%20Object%20Reference) (OtherBodyIndex :type Integer))
  ;[0.15 0.15 0.15 0.5] Display Widget
  (bind _asbp_third_person_character (Utilities|Casting|CastToBP_ThirdPersonCharacter OtherActor))
  (if (Variables|/Game/ThirdPerson/Blueprints/BP_ThirdPersonCharacter.BP_ThirdPersonCharacter_C|GetnightVisionUnlocked _asbp_third_person_character)
    (Widget|RemovefromParent (Variables|Default|GetNewVar))))

(event EventBeginPlay
  ;[0.15 0.15 0.15 0.5] Display Widget
  (bind _returnvalue (UserInterface|CreateWidget "/Game/Widgets/W_Interact.W_Interact_C"))
  (bind _output_get (Variables|Default|SetNewVar _returnvalue))
  (Variables|/Game/Widgets/W_Interact.W_Interact_C|SetPromptText _output_get "Press 'E' to open hatch"))

(event EventInteract
  (Actor|DestroyActor))

(fn ConstructionScript)

(fn ReturnText
  (return ""))